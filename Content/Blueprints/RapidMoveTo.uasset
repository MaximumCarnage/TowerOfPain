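; RapidMoveTo is a behavior tree task that sends an enemy pawn after its target and starts its attack on arrival.
; On execute it caches the EnemyAI controller, flags the Enemy_Base_BP pawn as aggroed, then runs AIMoveTo toward the TargetToFollow blackboard actor.
; On reaching the target it sets IsAttacking and finishes successfully; a failed move has no handler, so the task never finishes in that case.
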(event `self.ReceiveExecute`
  (params (OwnerActor :type "Actor Object Reference"))
  (if (not (!= (`self.AI_Control_Ref`) null))
    (bind _asenemy_ai (cast `/Game/Blueprints/EnemyAI` OwnerActor))
    (set `self.AI_Control_Ref` _asenemy_ai))
  (bind _asenemy_ai_2 (cast `/Game/Blueprints/EnemyAI` OwnerActor))
  (bind _asenemy_base_bp (cast `/Game/Blueprints/Enemy_Base_BP` (`Controller.K2_GetPawn` _asenemy_ai_2)))
  (set `/Game/Blueprints/Enemy_Base_BP.Aggro` true _asenemy_base_bp)
  (`|AIMoveTo` (`Controller.K2_GetPawn` (`self.AI_Control_Ref`)) (0.0 0.0 0.0) (`BTFunctionLibrary.GetBlackboardValueAsActor` (`self.TargetToFollow`)) 50.0
    (:`OnSuccess`
      (`KismetSystemLibrary.PrintString` "Reached Player")
      (bind _asenemy_ai_3 (cast `/Game/Blueprints/EnemyAI` (`self.AI_Control_Ref`)))
      (bind _asenemy_base_bp_2 (cast `/Game/Blueprints/Enemy_Base_BP` (`Controller.K2_GetPawn` _asenemy_ai_3)))
      (set `/Game/Blueprints/Enemy_Base_BP.isAttacking` true _asenemy_base_bp_2)
      (`self.FinishExecute` true))))