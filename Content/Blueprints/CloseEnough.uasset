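; Behavior Tree decorator for the enemy AI that gates a branch on distance to the follow target.
; It casts the owner to EnemyAI, then measures the distance from its controlled pawn to the TargetToFollow Blackboard actor.
; Despite the CloseEnough name, the check passes when that distance is at least AcceptableDistance, meaning the pawn is not yet inside that range.
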(fn `PerformConditionCheck`
  (params (OwnerActor :type "Actor Object Reference"))
  (returns (ReturnValue :type Boolean))
  (bind _asenemy_ai (cast `/Game/Blueprints/EnemyAI` OwnerActor))
  (set `self.AI_control_Ref` _asenemy_ai)
  (return (>= (`KismetMathLibrary.VSize` (- (`Actor.K2_GetActorLocation` (`BTFunctionLibrary.GetBlackboardValueAsActor` (`self.TargetToFollow`))) (`Actor.K2_GetActorLocation` (`Controller.K2_GetPawn` (`self.AI_control_Ref`))))) (`self.AcceptableDistance`))))