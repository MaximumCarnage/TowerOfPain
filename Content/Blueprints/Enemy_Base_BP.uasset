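; Base enemy Blueprint that handles health, damage and death.
; Health starts at its maximum on BeginPlay, and a custom TakeDamage function subtracts from it and sets an InPain flag while the enemy is alive.
; At zero or below it sets IsDead, unpossesses the AI controller and disables capsule collision.
; InPain is never cleared in this file, and Tick and overlap events are empty.
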(event `self.ReceiveBeginPlay`
  (set `self.Current_Health` (`self.Max_Health`)))

(event `self.ReceiveActorBeginOverlap`
  (params (OtherActor :type "Actor Object Reference")))

(event `self.ReceiveTick`
  (params (DeltaSeconds :type "Float (single-precision)")))

(fn `TakeDamage`
  (params (DamageInflicted :type Integer))
  (if (not (`self.isDead`))
    (set `self.InPain` true)
    (set `self.Current_Health` (- (`self.Current_Health`) DamageInflicted))
    (`/Engine/EditorBlueprintResources/StandardMacros.CompareInt` (`self.Current_Health`)
      (:`==`
        _)
      (:`<`
        _))
    (set `self.isDead` true)
    (`Controller.UnPossess` (`AIBlueprintHelperLibrary.GetAIController` self))
    (`PrimitiveComponent.SetCollisionEnabled` (`self.CapsuleComponent`) "NoCollision")))

(fn `UserConstructionScript`)