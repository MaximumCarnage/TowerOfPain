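; AI controller for enemy pawns that runs a behavior tree chosen by the enemy's type.
; On BeginPlay it sets up the EnemyBlackBoard, stores the pawn's spawn position as HomeLocation, and picks the Parasyte, Zombie, Bull or Death Mother tree.
; Each Tick it casts its Owner to Enemy_Base_BP and, if that enemy is dead, prints a debug message and unpossesses.
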(event `self.ReceiveBeginPlay`
  (bind _returnvalue (`self.K2_GetPawn`))
  (`self.UseBlackboard` "/Game/Models/Parasyte/EnemyBlackBoard.EnemyBlackBoard")
  (`BlackboardComponent.SetValueAsVector` (`AIBlueprintHelperLibrary.GetBlackboard` self) (`self.HomeLocation`) (`self.K2_GetActorLocation` _returnvalue))
  (bind _asenemy_base_bp (cast `/Game/Blueprints/Enemy_Base_BP` _returnvalue))
  (switch `/Game/Models/Parasyte/EnemyTypes` (`/Game/Blueprints/Enemy_Base_BP.EnemyType` _asenemy_base_bp)
    (:`NewEnumerator0`
      (`self.RunBehaviorTree` "/Game/Models/Parasyte/Para_BT.Para_BT"))
    (:`NewEnumerator1`
      (`self.RunBehaviorTree` "/Game/Models/Zombie/ZombieBT.ZombieBT"))
    (:`NewEnumerator3`
      (`self.RunBehaviorTree` "/Game/Models/Bull/Bull_BT.Bull_BT"))
    (:`NewEnumerator4`
      (`self.RunBehaviorTree` "/Game/Models/DeathMother/DeathMother_BT.DeathMother_BT"))))

(event `self.ReceiveTick`
  (params (DeltaSeconds :type "Float (single-precision)"))
  (bind _asenemy_base_bp (cast `/Game/Blueprints/Enemy_Base_BP` (`self.GetOwner`)))
  (if (`/Game/Blueprints/Enemy_Base_BP.isDead` _asenemy_base_bp)
    (`KismetSystemLibrary.PrintString` "IBeDead")
    (`self.UnPossess`)))

(fn `UserConstructionScript`)